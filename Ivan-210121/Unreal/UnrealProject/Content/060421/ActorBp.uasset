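; ActorBp is an actor whose Robot component changes its material when the player pawn is nearby.
; BeginPlay creates a dynamic material instance from Robot_Inst on the Robot component and stores it.
; Each Tick measures the distance to the player pawn and sets the Intensity scalar parameter on or off around a fixed radius threshold.
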(event EventBeginPlay
  (bind _returnvalue (Rendering|Material|CreateDynamicMaterialInstance (Variables|Default|GetRobot) 0 "/Game/060421/Robot_Inst.Robot_Inst" "None" :!class /Script/Engine.PrimitiveComponent))
  (Variables|Default|SetRobotMaterial _returnvalue))

(event Collision|EventActorBeginOverlap
  (params (OtherActor :type Actor%20Object%20Reference)))

(event EventTick
  (params (DeltaSeconds :type Float%20%28single-precision%29))
  (if (< (Math|Vector|Distance(Vector) (Transformation|GetActorLocation) (Transformation|GetActorLocation (Game|Player|GetPlayerPawn 0))) 5e+02)
    (Rendering|Material|SetScalarParameterValue (Variables|Default|GetRobotMaterial) "Intensity" 1.0 :!class /Script/Engine.MaterialInstanceDynamic)
    (else
      (Rendering|Material|SetScalarParameterValue (Variables|Default|GetRobotMaterial) "Intensity" 0.0 :!class /Script/Engine.MaterialInstanceDynamic))))

(fn ConstructionScript)